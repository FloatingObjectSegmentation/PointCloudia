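; Pointer actor that orients itself once at BeginPlay along the line between two cubes in the level.
; It gathers every StaticMeshActor whose display name contains "Cube" and stores their locations in an array.
; It then builds a rotation whose forward axis runs from the second stored location toward the first, leaving right and up zeroed, without checking that two cubes exist.
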(event `self.ReceiveBeginPlay`
  (bind _outactors (`GameplayStatics.GetAllActorsOfClass` "/Script/Engine.StaticMeshActor"))
  (for _array_element _outactors
    ;[1 1 1] Add cubes to array
    (if (`KismetStringLibrary.Contains` (`KismetSystemLibrary.GetDisplayName` _array_element) "Cube")
      (`KismetArrayLibrary.Array_Add` (`self.Locations`) (`self.K2_GetActorLocation` _array_element))))
  (`self.K2_SetActorRotation` (`KismetMathLibrary.MakeRotationFromAxes` (- (`|GetArrayItem` (`self.Locations`)) (`|GetArrayItem` (`self.Locations`) 1)))))

(fn `UserConstructionScript`)