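; StartingPointer is an actor Blueprint that serves as a keyboard control for an AugmentationStarter, apparently to orient and launch an augmentation.
; BeginPlay enables input from player controller 0 so the actor receives key presses directly.
; U and O call TransformYaw on the AugmentationStarter with opposite signs, and Space Bar calls StartAugmentation.
; Tick and overlap events are disabled, and the construction script only calls its parent.
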(event `Key|U`
  (params (Key :type "Key Structure"))
  (:`Pressed`
    (`AugmentationStarterComponent.TransformYaw` (`self.AugmentationStarter`) 1)))

(event `Key|O`
  (params (Key :type "Key Structure"))
  (:`Pressed`
    (`AugmentationStarterComponent.TransformYaw` (`self.AugmentationStarter`) -1)))

(event `Key|SpaceBar`
  (params (Key :type "Key Structure"))
  (:`Pressed`
    (`AugmentationStarterComponent.StartAugmentation` (`self.AugmentationStarter`))))

(event `self.ReceiveBeginPlay`
  (`parent.ReceiveBeginPlay`)
  (`self.EnableInput` (`GameplayStatics.GetPlayerController` 0)))

(fn `UserConstructionScript`
  (`parent.UserConstructionScript`))